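; Pinball-style bumper actor that knocks a BP_Ball away when the ball overlaps it.
; The bump applies a velocity-change impulse along the direction from bumper to ball and plays an attached hit sound.
; A timeline drives the mechanism's vertical offset, point light intensity and top material's emissive boost from one alpha.
; The construction script creates the dynamic material instance for that glow.
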(event Custom|bump
  (params (ball :type BP%20Ball%20Object%20Reference))
  (Physics|AddImpulse (Variables|/Game/blueprints/BP_Ball.BP_Ball_C|Getball ball) (* (Math|Vector|GetUnitDirection(Vector) (Transformation|GetActorLocation) (Transformation|GetActorLocation ball)) 2.5e+03) "None" true)
  (Audio|SpawnSoundAttached "/Game/assets/sounds/BumperHit.BumperHit" (Variables|Default|Getbumpermesh))
  (bind _bumpalfa (Timeline|bumplerp PlayFromStart)
    (:Update
      (Transformation|SetRelativeLocation (Variables|Default|GetBupermecanism) (Math|Vector|Lerp(Vector) "0, 0, 0" "0, 0,-70.000000" _bumpalfa) false false)
      (Rendering|Components|Light|SetIntensity (Variables|Default|GetPointLight) (Math|Float|Lerp 0.0 5e+03 _bumpalfa))
      (Rendering|Material|SetScalarParameterValue (Variables|Default|GetbumpertopMID) "emessivebost" (Math|Float|Lerp 0.0 2e+02 _bumpalfa) :!class /Script/Engine.MaterialInstanceDynamic))))

(event EventBeginPlay)

(event Collision|EventActorBeginOverlap
  (params (OtherActor :type Actor%20Object%20Reference))
  (bind _asbp_ball (Utilities|Casting|CastToBP_Ball OtherActor))
  (CallFunction|Bump _asbp_ball))

(event EventTick
  (params (DeltaSeconds :type Float%20%28single-precision%29)))

(fn ConstructionScript
  (bind _returnvalue (Rendering|Material|CreateDynamicMaterialInstance (Variables|Default|Getbumpermesh) 1 0 :!class /Script/Engine.PrimitiveComponent))
  (Variables|Default|SetbumpertopMID _returnvalue)
  (Rendering|Material|SetScalarParameterValue (Variables|Default|GetbumpertopMID) "None" 0.0 :!class /Script/Engine.MaterialInstanceDynamic))